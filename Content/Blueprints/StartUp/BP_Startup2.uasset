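; BP_Startup2 is an actor that continuously spins three static mesh components about their vertical axis, each at a different speed.
; Each Tick adds a fixed yaw step to every mesh's relative rotation and zeroes pitch and roll, so speed depends on frame rate.
; Disconnected nodes for rotating and moving the whole actor, and for an alternate mesh spin, never run.
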(event `self.ReceiveTick`
  (params (DeltaSeconds :type "Float (single-precision)"))
  (bind _staticmesh (`self.StaticMesh`))
  (bind _staticmeshcomponent (`self.StaticMeshComponent`))
  (bind _staticmesh1 (`self.StaticMesh1`))
  (bind (_relativerotation_roll _relativerotation_pitch _relativerotation_yaw) (`KismetMathLibrary.BreakRotator` (`SceneComponent.RelativeRotation` _staticmesh1)))
  (bind (_relativerotation_roll_2 _relativerotation_pitch_2 _relativerotation_yaw_2) (`KismetMathLibrary.BreakRotator` (`SceneComponent.RelativeRotation` _staticmesh)))
  (bind (_relativerotation_roll_3 _relativerotation_pitch_3 _relativerotation_yaw_3) (`KismetMathLibrary.BreakRotator` (`SceneComponent.RelativeRotation` _staticmeshcomponent)))
  (`|ExecutionSequence`
    (:`then_0`
      (`SceneComponent.K2_SetRelativeRotation` _staticmeshcomponent (`KismetMathLibrary.MakeRotator` 0.0 0.0 (+ _relativerotation_yaw_3 1.0)) false false))
    (:`then_1`)
    (:`then_2`
      (`SceneComponent.K2_SetRelativeRotation` _staticmesh1 (`KismetMathLibrary.MakeRotator` 0.0 0.0 (+ _relativerotation_yaw 2.5)) false false))
    (:`then_3`
      (`SceneComponent.K2_SetRelativeRotation` _staticmesh (`KismetMathLibrary.MakeRotator` 0.0 0.0 (+ _relativerotation_yaw_2 5.0)) false false))))

(event `self.ReceiveBeginPlay`)

(fn `UserConstructionScript`)